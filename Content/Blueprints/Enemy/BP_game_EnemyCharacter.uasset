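; Enemy character Blueprint that detects the player by sight and alerts its AI.
; When PawnSensing sees a BP_game_PlayerCharacter with the player entity type, it sets the HasSeenPlayer blackboard key to drive the LookAtPlayer task.
; The key is never cleared here; an unused view-angle check for losing sight remains unconnected.
; BeginPlay also sets a DEBUG flag meant for debug lines.
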(event `self.ReceiveBeginPlay`
  ;[1 1 1] set this to true if you want to show debug lines
  (set `self.DEBUG` false))

(event `self.ReceiveTick`
  (params (DeltaSeconds :type "Float (single-precision)")))

(event `self.PawnSensing.OnSeePawn`
  (params (Pawn :type "Pawn Object Reference"))
  ;[1 1 1] Check if seen pawn is actually a player
  (bind _asbp_game_player_character (cast `/Game/Blueprints/Player/BP_game_PlayerCharacter` Pawn))
  (if (== (`KismetMathLibrary.Conv_ByteToInt` (`game_PlayerCharacter.entityType` _asbp_game_player_character)) (`KismetMathLibrary.Conv_ByteToInt` (`self.playerEntityType`)))
    ;[1 1 1] Change the "HasSeenPlayer" blackboard key to true (go to LookAtPlayer task)
    (`BlackboardComponent.SetValueAsBool` (`AIBlueprintHelperLibrary.GetBlackboard` (`AIBlueprintHelperLibrary.GetAIController` self)) "HasSeenPlayer" true)))

(fn `UserConstructionScript`)