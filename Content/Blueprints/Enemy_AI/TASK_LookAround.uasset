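; Behavior tree task that makes an enemy character look around by turning in place by a random angle.
; On execute, it casts the controlled pawn to the enemy character, then picks a random direction and angle, negating speed and target for counterclockwise turns.
; Tick yaws the root component at a constant speed, accumulates the degrees turned and finishes the task successfully once the target is reached.
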(event `self.ReceiveExecuteAI`
  (params (OwnerController :type "AIController Object Reference") (ControlledPawn :type "Pawn Object Reference"))
  (bind _asbp_game_enemy_character (cast `/Game/Blueprints/Enemy/BP_game_EnemyCharacter` ControlledPawn))
  ;[1 1 1] Set Defaults
  (bind _output_get (set `self.As BP Game Enemy Character` _asbp_game_enemy_character))
  (set `self.currentRotation` (`SceneComponent.K2_GetComponentRotation` (`game_EnemyCharacter.bodyMesh` _output_get)))
  (set `self.RotationSpeed` 70.0)
  (set `self.degreesToRotate` (`KismetMathLibrary.RandomFloatInRange` 45.0 180.0))
  (set `self.degreesAlreadyRotated` 0.0)
  ;[1 1 1] If MovesClockwise = false - make rotationSpeed and
  ; degreesToRotate negative for counterclockwise rotation
  (bind _output_get_2 (set `self.movesClockwise` (`KismetMathLibrary.RandomBool`)))
  (if (not _output_get_2)
    (set `self.RotationSpeed` (* -1.0 (`self.RotationSpeed`)))
    (set `self.degreesToRotate` (* -1.0 (`self.degreesToRotate`)))))

(event `self.ReceiveTick`
  (params (OwnerActor :type "Actor Object Reference") (DeltaSeconds :type "Float (single-precision)"))
  (bind _degreestorotate (`self.degreesToRotate`))
  (bind _degreesalreadyrotated (`self.degreesAlreadyRotated`))
  (bind _returnvalue (* DeltaSeconds (`self.RotationSpeed`)))
  ;[1 1 1] Rotate ROOT COMPONENT according to rotation speed
  (`SceneComponent.K2_AddWorldRotation` (`Actor.RootComponent` (`self.As BP Game Enemy Character`)) (`KismetMathLibrary.MakeRotator` 0.0 0.0 _returnvalue) false false)
  ;[1 1 1] Update already rotated amount
  (set `self.degreesAlreadyRotated` (+ _returnvalue (`self.degreesAlreadyRotated`)))
  ;[1 1 1] If moving clockwise - check if already rotated degrees >= target rotation degrees (they are positive)
  ; if counterclockwise - check if they are <= (they are negative)
  (if (`self.movesClockwise`)
    (if (>= _degreesalreadyrotated _degreestorotate)
      (`self.FinishExecute` true :!label _label))
    (elif (<= _degreesalreadyrotated _degreestorotate)
      (goto _label))))