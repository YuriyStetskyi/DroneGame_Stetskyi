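; Behavior tree task that makes a turret enemy track and shoot the player it has detected.
; On execute it turns the detection indicator red; each tick it checks sight radius and line-traces to the player.
; With clear sight it yaws the body, pitches the gun and fires through the AI controller, throttled by a one-second Delay.
; Losing the player clears HasSeenPlayer on the blackboard, restores the green indicator and finishes the task.
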(event `self.ReceiveExecuteAI`
  (params (OwnerController :type "AIController Object Reference") (ControlledPawn :type "Pawn Object Reference"))
  ;[1 1 1] Set BP player character
  (bind _asbp_game_enemy_character (cast `/Game/Blueprints/Enemy/BP_game_EnemyCharacter` ControlledPawn))
  (bind _output_get (set `self.As BP Game Enemy Character` _asbp_game_enemy_character))
  ;[1 1 1] Change player detection indicator color to RED (because detected)
  (`PrimitiveComponent.SetMaterial` (`game_EnemyCharacter.playerDetectionIndicatorMesh` _output_get) 0 "/Game/Visuals/Materials/Enemy/color_playerDETECTED.color_playerDETECTED")
  ;[1 1 1] If in debug mode - draw lines
  (if (`/Game/Blueprints/Enemy/BP_game_EnemyCharacter.DEBUG` (`self.As BP Game Enemy Character`))
    (set `self.Draw lines` "ForDuration")
    (else
      (set `self.Draw lines` "None"))))

(event `self.ReceiveTickAI`
  (params (OwnerController :type "AIController Object Reference") (ControlledPawn :type "Pawn Object Reference") (DeltaSeconds :type "Float (single-precision)"))
  (bind _returnvalue (`GameplayStatics.GetPlayerPawn` 0))
  (bind _returnvalue_2 (* DeltaSeconds 5.0))
  (bind _mesh (`Character.Mesh` (`self.As BP Game Enemy Character`)))
  (bind _returnvalue_3 (`SceneComponent.K2_GetComponentLocation` _mesh))
  (bind (_yaw _pitch) (`KismetMathLibrary.GetYawPitchFromVector` (`KismetMathLibrary.Conv_RotatorToVector` (`KismetMathLibrary.FindLookAtRotation` (`SceneComponent.K2_GetComponentLocation` (`Character.Mesh` (`self.As BP Game Enemy Character`))) (`SceneComponent.K2_GetComponentLocation` (`Actor.RootComponent` (`GameplayStatics.GetPlayerPawn` 0)))))))
  ;[1 1 1] TRUE if distance from player to enemy is > than pawn sensing ddistance
  (`/Engine/EditorBlueprintResources/StandardMacros.IsValid` _returnvalue
    (:`Is Valid`
      (if (> (`Actor.GetDistanceTo` _returnvalue ControlledPawn) (`PawnSensingComponent.SightRadius` (`/Game/Blueprints/Enemy/BP_game_EnemyCharacter.PawnSensing` (`self.As BP Game Enemy Character`))))
        ;[1 1 1] Set blackboard "HasSeenPlayer" key to false. (return to looking around task)
        (`BlackboardComponent.SetValueAsBool` (`AIBlueprintHelperLibrary.GetBlackboard` (`AIBlueprintHelperLibrary.GetAIController` (`self.As BP Game Enemy Character`))) "HasSeenPlayer" false :!label _label)
        ;[1 1 1] Change player detection indicator color back to GREEN (player no longer detected)
        (`PrimitiveComponent.SetMaterial` (`game_EnemyCharacter.playerDetectionIndicatorMesh` (`self.As BP Game Enemy Character`)) 0 "/Game/Visuals/Materials/Enemy/color_playerNOTDETECTED.color_playerNOTDETECTED")
        (`self.FinishExecute` true)
        (else
          ;[1 1 1] TRUE if player is behind an obstacle
          ;;[1 1 1] draw line in direction where turret is looking
          (`KismetSystemLibrary.LineTraceSingle` :`Start` _returnvalue_3 :`End` (+ _returnvalue_3 (* (`SceneComponent.GetForwardVector` _mesh) (1000.0 1000.0 1000.0))) :`TraceChannel` "TraceTypeQuery1" :`DrawDebugType` (`self.Draw lines`) :`DrawTime` _returnvalue_2)
          ;;[1 1 1] draw line from turret to player
          (bind _outhit (`KismetSystemLibrary.LineTraceSingle` _returnvalue_3 (`SceneComponent.K2_GetComponentLocation` (`Actor.RootComponent` (`GameplayStatics.GetPlayerPawn` 0))) "TraceTypeQuery1" false (`|MakeArray` (`self.As BP Game Enemy Character`) :!type "Actor Object Reference") (`self.Draw lines`) true (struct :`B` 1.0 :`A` 1.0) (struct :`G` 1.0 :`A` 1.0) _returnvalue_2))
          ;;[1 1 1] if hit actor is NOT a player
          (cast `/Game/Blueprints/Player/BP_game_PlayerCharacter` (`.HitActor` (`GameplayStatics.BreakHitResult` _outhit))
            (:`then`
              ;[1 1 1] Set body yaw to that rotation
              (bind _output_get (set `self.Rotator at player` (`KismetMathLibrary.MakeRotator` 0.0 0.0 _yaw)))
              (`SceneComponent.K2_SetWorldRotation` (`Actor.RootComponent` (`self.As BP Game Enemy Character`)) _output_get false false)
              ;[1 1 1] Set turret Pitch to that rotation
              (bind _output_get_2 (set `self.Rotator at player` (`KismetMathLibrary.MakeRotator` 0.0 _pitch)))
              (`SceneComponent.K2_SetRelativeRotation` (`game_EnemyCharacter.gunMesh` (`self.As BP Game Enemy Character`)) _output_get_2 false false)
              ;[1 1 1] Shoot every second
              (bind _asbp_game_enemy_aicontroller (cast `/Game/Blueprints/Enemy/BP_game_EnemyAIController` (`Pawn.GetController` (`self.As BP Game Enemy Character`))))
              (`KismetSystemLibrary.Delay` 1.0)
              (`game_EnemyAIController.ShootAtDirection` _asbp_game_enemy_aicontroller (`SceneComponent.GetForwardVector` (`game_EnemyCharacter.muzzleMesh` (`self.As BP Game Enemy Character`)))))
            (:`CastFailed`
              (goto _label))))))
    (:`Is Not Valid`
      (goto _label))))